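; BP_CubeSpawner is an actor that periodically spawns grabbable small cubes at its own transform until the first puzzle is complete.
; Tick accumulates delta time and spawns a Grabbable_SmallCube whenever the timer reaches SpawnInterval, then resets it.
; On BeginPlay it binds to the game state's Puzzle1Complete event, which disables actor tick to stop spawning.
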(event Custom|EventOnPuzzle1Complete
  ;[0.15 0.15 0.15 0.5] Disable tick if puzzle1 complete
  (Actor|Tick|SetActorTickEnabled false))

(event EventBeginPlay
  (bind _asgame_state_base (Utilities|Casting|CastToGameStateBase (Game|GetGameState)))
  (EventDispatchers|BindEventtoPuzzle1Complete _asgame_state_base (delegate Custom|EventOnPuzzle1Complete)))

(event Collision|EventActorBeginOverlap
  (params (OtherActor :type Actor%20Object%20Reference)))

(event EventTick
  (params (DeltaSeconds :type Float%20%28single-precision%29))
  ;[0.15 0.15 0.15 0.5] Spawn a small cube on set interval
  (bind _output_get (Variables|Default|Settimer (+ DeltaSeconds (Variables|Default|Gettimer))))
  (if (>= _output_get (Variables|Default|GetspawnInterval))
    (Game|SpawnActorfromClass "/Game/VRTemplate/Blueprints/Grabbable_SmallCube.Grabbable_SmallCube_C" (Transformation|GetActorTransform) "Undefined" "MultiplyWithRoot" 0 0)
    (Variables|Default|Settimer 0.0)))

(fn ConstructionScript)