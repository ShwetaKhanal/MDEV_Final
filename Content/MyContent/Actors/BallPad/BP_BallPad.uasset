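; BP_BallPad is a puzzle pad actor that consumes balls and signals the game state when the second puzzle is solved.
; When a BP_Ball overlaps the Collider, the pad destroys it, increments BallCount and scales the red plane in X and Y by BallCount over FillBallCount.
; The solve event, EventPuzzle2Solved, fires at a hardcoded count of three or more, independent of FillBallCount.
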(event OnComponentBeginOverlap(Collider)
  (params (OverlappedComponent :type Primitive%20Component%20Object%20Reference) (OtherActor :type Actor%20Object%20Reference) (OtherComp :type Primitive%20Component%20Object%20Reference) (OtherBodyIndex :type Integer) (bFromSweep :type Boolean) (SweepResult :type Hit%20Result%20Structure%20%28by%20ref%29))
  (if (== (Utilities|GetClass OtherActor) "/Game/MyContent/Actors/Ball/BP_Ball.BP_Ball_C")
    (Actor|DestroyActor OtherActor)
    (bind _result (Math|Integer|IncrementInt (Variables|Default|GetBallCount))
      (:%20%20
        (CallFunction|ScaleRedPlane)
        (if (>= _result 3)
          (bind _asgame_state_base (Utilities|Casting|CastToGameStateBase (Game|GetGameState)))
          (Default|EventPuzzle2Solved _asgame_state_base))))))

(event EventBeginPlay)

(event Collision|EventActorBeginOverlap
  (params (OtherActor :type Actor%20Object%20Reference)))

(event EventTick
  (params (DeltaSeconds :type Float%20%28single-precision%29)))

(fn ConstructionScript)

(fn ScaleRedPlane
  (bind _ballcount (Variables|Default|GetBallCount))
  (bind _fillballcount (Variables|Default|GetFillBallCount))
  (bind _returnvalue (Math|Conversions|ToFloat(Integer) _ballcount))
  (bind _returnvalue_2 (Math|Conversions|ToFloat(Integer) _fillballcount))
  (bind _returnvalue_3 (Math|Float|SafeDivide _returnvalue _returnvalue_2))
  ;[0.15 0.15 0.15 0.5] Show red plane based on how many balls have been provided
  (Transformation|SetRelativeScale3D (Variables|Default|GetRedPlane) (Math|Vector|MakeVector _returnvalue_3 _returnvalue_3 1.0)))