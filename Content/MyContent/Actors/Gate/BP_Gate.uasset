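; BP_Gate is a gate actor that lifts open once both puzzles are solved.
; On BeginPlay it binds to the Puzzle 1 and Puzzle 2 completion events on the game state, each of which rechecks both solved flags.
; When both are set, Tick raises the Cube component at LiftSpeed with a teleporting relative move, counting LiftAmount down until it runs out.
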(event Custom|EventPuzzleComplete
  (bind _gamestate (Variables|Default|GetGameState))
  ;[0.15 0.15 0.15 0.5] If both puzzles are complete
  (if (and (Variables|/Game/Blueprints/GameStateBase.GameStateBase_C|GetbIsPuzzle1Solved _gamestate) (Variables|/Game/Blueprints/GameStateBase.GameStateBase_C|GetbIsPuzzle2Solved _gamestate))
    (Variables|Default|SetbIsOpening true)))

(event EventBeginPlay
  (bind _asgame_state_base (Utilities|Casting|CastToGameStateBase (Game|GetGameState)))
  (bind _output_get (Variables|Default|SetGameState _asgame_state_base))
  (EventDispatchers|BindEventtoPuzzle1Complete _output_get (delegate Custom|EventPuzzleComplete))
  (EventDispatchers|BindEventtoPuzzle2Complete _output_get (delegate Custom|EventPuzzleComplete)))

(event Collision|EventActorBeginOverlap
  (params (OtherActor :type Actor%20Object%20Reference)))

(event EventTick
  (params (DeltaSeconds :type Float%20%28single-precision%29))
  (bind _liftspeed (Variables|Default|GetLiftSpeed))
  (bind _returnvalue (* DeltaSeconds _liftspeed))
  (if (Variables|Default|GetbIsOpening)
    (if (<= (Variables|Default|GetLiftAmount) 0.0)
      ;[0.15 0.15 0.15 0.5] Lift Complete
      (Variables|Default|SetbIsOpening false)
      (else
        (Transformation|AddRelativeLocation (Variables|Default|GetCube) (Math|Vector|MakeVector 0.0 0.0 _returnvalue) false true)
        (Variables|Default|SetLiftAmount (- (Variables|Default|GetLiftAmount) _returnvalue))))))

(fn ConstructionScript)