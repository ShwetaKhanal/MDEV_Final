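; Cube receiver actor for puzzle 1 that consumes small grabbable cubes and reports the puzzle solved once its depletion timer runs out.
; Tick advances the timer through UpdateMaterial, which also drives the cube material's LerpFactor from elapsed time over DepletionDelay.
; A small cube overlapping the collider is destroyed and resets the timer.
; Once the delay is reached, Puzzle1Solved is called on the GameState every tick until a reset.
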(event OnComponentBeginOverlap(Collider)
  (params (OverlappedComponent :type Primitive%20Component%20Object%20Reference) (OtherActor :type Actor%20Object%20Reference) (OtherComp :type Primitive%20Component%20Object%20Reference) (OtherBodyIndex :type Integer) (bFromSweep :type Boolean) (SweepResult :type Hit%20Result%20Structure%20%28by%20ref%29))
  ;[0.15 0.15 0.15 0.5] When hit by small cube destroy it and reset the depletion timer
  (if (== (Utilities|GetClass OtherActor) "/Game/VRTemplate/Blueprints/Grabbable_SmallCube.Grabbable_SmallCube_C")
    (Actor|DestroyActor OtherActor)
    (Variables|Default|SetdepletionTimer 0.0)))

(event EventBeginPlay)

(event Collision|EventActorBeginOverlap
  (params (OtherActor :type Actor%20Object%20Reference)))

(event EventTick
  (params (DeltaSeconds :type Float%20%28single-precision%29))
  (bind _depletiontimer (CallFunction|UpdateMaterial DeltaSeconds))
  ;[0.15 0.15 0.15 0.5] If Depletion timer ran longer than delay, start puzzle 1 complete
  (if (>= _depletiontimer (Variables|Default|GetdepletionDelay))
    (bind _asgame_state_base (Utilities|Casting|CastToGameStateBase (Game|GetGameState)))
    (Default|Puzzle1Solved _asgame_state_base)))

(fn ConstructionScript)

(fn UpdateMaterial
  (params (DeltaTime :type Float%20%28double-precision%29))
  ;[0.15 0.15 0.15 0.5] Update Material color and timer
  (bind _output_get (Variables|Default|SetdepletionTimer (+ DeltaTime (Variables|Default|GetdepletionTimer))))
  (Rendering|Material|SetScalarParameterValueonMaterials (Variables|Default|GetCube) "LerpFactor" (/ _output_get (Variables|Default|GetdepletionDelay)))
  (return _output_get))