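; Game state Blueprint for a VR puzzle game that tracks the countdown, two puzzles and game over.
; On BeginPlay it binds to the VRPawn's PlayerDied event, which runs GameOver to set IsGameOver and signal GameIsOver.
; Tick decrements TimeLimit until game over, calling TimeUp every frame it is at or below zero, without triggering GameOver itself.
; Each puzzle-solved event sets its flag and signals completion.
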(event Custom|Puzzle1Solved
  ;[0.15 0.15 0.15 0.5] When puzzle 1 is solved, signal puzzle1 complete
  (Variables|Default|SetbIsPuzzle1Solved true)
  (Default|CallPuzzle1Complete))

(event Custom|EventPuzzle2Solved
  ;[0.15 0.15 0.15 0.5] When puzzle 2 is solved, signal puzzle 2 complete
  (Variables|Default|SetbIsPuzzle2Solved true)
  (Default|CallPuzzle2Complete))

(event Custom|Event%20PlayerDied
  ;[0.15 0.15 0.15 0.5] GameOver when Player Died
  (CallFunction|GameOver))

(event EventBeginPlay
  ;[0.15 0.15 0.15 0.5] GameOver when Player Died
  (bind _asvrpawn (Utilities|Casting|CastToVRPawn (Game|Player|GetPlayerPawn 0)))
  (EventDispatchers|BindEventtoPlayerDied _asvrpawn (delegate Custom|Event%20PlayerDied)))

(event EventTick
  (params (DeltaSeconds :type Float%20%28single-precision%29))
  ;[0.15 0.15 0.15 0.5] Countdown timer
  (if (not (Variables|Default|GetbIsGameOver))
    (bind _output_get (Variables|Default|SetTimeLimit (- (Variables|Default|GetTimeLimit) DeltaSeconds)))
    (if (<= _output_get 0.0)
      (Default|CallTimeUp))))

(fn ConstructionScript)

(fn GameOver
  (Variables|Default|SetbIsGameOver true)
  (Default|CallGameIsOver))